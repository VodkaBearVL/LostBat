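; BP_BatManager chooses which bat relative the 2D side-scroller player character has as its current objective.
; On BeginPlay it caches the character, then CurrentTarget gathers all BP_BatRelative actors and assigns a random one to the character's CurrentObjective.
; UpdateTarget destroys the character's FoundRelative, clears the list and runs CurrentTarget again to pick the next objective.
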(event Custom|CurrentTarget
  (bind _outactors (Actor|GetAllActorsOfClass "/Game/MY_BP/BP_BatRelative.BP_BatRelative_C"))
  (Variables|Default|SetBatsToFind _outactors)
  (Variables|/Game/MY_BP/2DSideScrollerCharacter.2DSideScrollerCharacter_C|SetCurrentObjective (Variables|Default|GetChar) (Utilities|Array|Get(acopy) (Variables|Default|GetBatsToFind) (Math|Random|RandomIntegerinRange 0 (Utilities|Array|LastIndex (Variables|Default|GetBatsToFind))))))

(event Custom|UpdateTarget
  (Actor|DestroyActor (Variables|/Game/MY_BP/2DSideScrollerCharacter.2DSideScrollerCharacter_C|GetFoundRelative (Variables|Default|GetChar)))
  (Utilities|Array|Clear (Variables|Default|GetBatsToFind))
  (CallFunction|CurrentTarget))

(event EventBeginPlay
  (bind _as2dside_scroller_character (Utilities|Casting|CastTo2DSideScrollerCharacter (Game|GetPlayerCharacter 0)))
  (Variables|Default|SetChar _as2dside_scroller_character)
  (CallFunction|CurrentTarget))

(fn ConstructionScript)